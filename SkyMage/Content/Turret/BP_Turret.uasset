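; Turret actor that turns toward a Player-tagged actor inside its sphere and shoots a Niagara fire-cube effect.
; Sphere overlap starts looping timers that yaw the Arrow toward the target and line-trace to it, reactivating the effect on a player hit.
; Leaving the sphere clears both timers and deactivates the effect.
; A particle data event calls ApplyDamage per entry, but no damaged actor is wired.
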(event `self.Sphere.OnComponentBeginOverlap`
  (params (OverlappedComponent :type "PrimitiveComponent Object Reference") (OtherActor :type "Actor Object Reference") (OtherComp :type "PrimitiveComponent Object Reference") (OtherBodyIndex :type Integer) (bFromSweep :type Boolean) (SweepResult :type "HitResult Structure (by ref)"))
  (bind _niagara (`self.Niagara`))
  ;[0 0 0.8739 0.5] When the turret sees the player (IT HAS EYES???)
  (`/Engine/EditorBlueprintResources/StandardMacros.IsValid` OtherActor
    (:`Is Valid`
      (if (`self.ActorHasTag` OtherActor "Player")
        (set `self.Target` OtherActor)
        (`self.Track Target`)
        (`NiagaraComponent.SetAsset` _niagara "/Game/VFX/NA_Systems/NS_FireCubes.NS_FireCubes" true)
        (`ActorComponent.Activate` _niagara false)))))

(event `self.Sphere.OnComponentEndOverlap`
  (params (OverlappedComponent :type "PrimitiveComponent Object Reference") (OtherActor :type "Actor Object Reference") (OtherComp :type "PrimitiveComponent Object Reference") (OtherBodyIndex :type Integer))
  ;[0.8307 0 0 0.5] When turret can't see the player (might be blind)
  (`/Engine/EditorBlueprintResources/StandardMacros.IsValid` OtherActor
    (:`Is Valid`
      (if (`self.ActorHasTag` OtherActor "Player")
        (`self.Target`
          (:`then`
            (`KismetSystemLibrary.K2_ClearAndInvalidateTimerHandle` (`self.TimerRef`))
            (`KismetSystemLibrary.K2_ClearAndInvalidateTimerHandle` (`self.FireTimer`))
            (`ActorComponent.Deactivate` (`self.Niagara`)))
          (:`else`))))))

(event `self.ReceiveParticleData`
  (params (Data :type "Array of BasicParticleData Structure (by ref)") (NiagaraSystem :type "NiagaraSystem Object Reference") (SimulationPositionOffset :type "Vector Structure (by ref)"))
  (for _array_element Data
    (`GameplayStatics.ApplyDamage` null 10.0 null null "/Script/Engine.DamageType" :!label _label))
  (goto _label))

(event `Track Target`
  ;[0 0.7812 0 0.4043] Turret Rotation
  (bind _returnvalue (`KismetSystemLibrary.K2_SetTimerDelegate` (delegate `Move turret`) 0.05 true true))
  (set `self.TimerRef` _returnvalue)
  (bind _returnvalue_2 (`KismetSystemLibrary.K2_SetTimerDelegate` (delegate `Shoot Target`) 0.001 true true))
  (set `self.FireTimer` _returnvalue_2))

(event `Move turret`
  (bind _target (`self.Target`))
  (bind _arrow (`self.Arrow`))
  (bind (_returnvalue_roll _returnvalue_pitch _returnvalue_yaw) (`KismetMathLibrary.BreakRotator` (`KismetMathLibrary.RInterpTo` (`SceneComponent.GetSocketRotation` _arrow "None") (`KismetMathLibrary.FindLookAtRotation` (`self.K2_GetActorLocation`) (`self.K2_GetActorLocation` _target)) (`GameplayStatics.GetWorldDeltaSeconds`) 100.0)))
  ;[0 0.7812 0 0.4043] Turret Rotation
  (`/Engine/EditorBlueprintResources/StandardMacros.IsValid` _target
    (:`Is Valid`
      (`SceneComponent.K2_SetRelativeRotation` _arrow (`KismetMathLibrary.MakeRotator` 0.0 0.0 _returnvalue_yaw) false false))))

(event `Shoot Target`
  (bind _niagara (`self.Niagara`))
  ;[1 0.265 0] arson (Shooting the Fire)
  (bind (_outhit _returnvalue) (`KismetSystemLibrary.LineTraceSingle` :`Start` (+ (`self.K2_GetActorLocation`) (0.0 0.0 0.0)) :`End` (`self.K2_GetActorLocation` (`self.Target`)) :`TraceChannel` "TraceTypeQuery1" :`TraceColor` (struct :`G` 1.0 :`A` 1.0) :`TraceHitColor` (struct :`R` 1.0 :`A` 1.0)))
  (if _returnvalue
    (if (`self.ActorHasTag` (`.HitActor` (`GameplayStatics.BreakHitResult` _outhit)) "Player")
      (`NiagaraComponent.SetAsset` _niagara "/Game/VFX/NA_Systems/NS_FireCubes.NS_FireCubes" true)
      (`ActorComponent.Activate` _niagara false))))

(fn `UserConstructionScript`)